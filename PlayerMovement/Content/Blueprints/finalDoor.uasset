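; Final door actor that swings open when a key reaches it.
; While Locked, a BoxCollision overlap checks for an actor tagged "Key" or a component tagged "FinalKey".
; A match passes a DoOnce to play the DoorMovement timeline, which rotates the mesh's yaw and clears Locked.
; The DoorOpenLevelCall event reaches the same check only through a constant-true branch's False side, so it never opens the door.
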(event OnComponentBeginOverlap(BoxCollision)
  (params (OverlappedComponent :type Primitive%20Component%20Object%20Reference) (OtherActor :type Actor%20Object%20Reference) (OtherComp :type Primitive%20Component%20Object%20Reference) (OtherBodyIndex :type Integer) (bFromSweep :type Boolean) (SweepResult :type Hit%20Result%20Structure%20%28by%20ref%29))
  (if (Variables|Default|GetLocked)
    (if (or (Actor|ActorHasTag OtherActor "Key") (Components|ComponentHasTag OtherComp "FinalKey"))
      (Variables|Default|SetLocked true)
      (Utilities|FlowControl|DoOnce false
        (:Completed
          (bind _openclose (Timeline|DoorMovement Play)
            (:Update
              (Transformation|SetRelativeRotation (Variables|Debug|GetStaticMeshComponent) (Math|Rotator|MakeRotator 0.0 0.0 _openclose) false false)
              (Variables|Default|SetLocked false))))))))

(event Custom|DoorOpenLevelCall
  (if (not true)
    (if (Variables|Default|GetLocked)
      (if (or (Actor|ActorHasTag (stale OnComponentBeginOverlap(BoxCollision) OtherActor) "Key") (Components|ComponentHasTag (stale OnComponentBeginOverlap(BoxCollision) OtherComp) "FinalKey"))
        (Variables|Default|SetLocked true)
        (Utilities|FlowControl|DoOnce false
          (:Completed
            (bind _openclose (Timeline|DoorMovement Play)
              (:Update
                (Transformation|SetRelativeRotation (Variables|Debug|GetStaticMeshComponent) (Math|Rotator|MakeRotator 0.0 0.0 _openclose) false false)
                (Variables|Default|SetLocked false)))))))))

(event EventBeginPlay)

(event Collision|EventActorBeginOverlap
  (params (OtherActor :type Actor%20Object%20Reference)))

(event EventTick
  (params (DeltaSeconds :type Float%20%28single-precision%29)))

(fn ConstructionScript)